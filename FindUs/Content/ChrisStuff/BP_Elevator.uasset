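; Elevator actor that opens a floor selection widget on interaction and travels vertically between three floors.
; Interact locks further use, shows WBP_FloorSelect and switches to UI-only input with the mouse cursor.
; MoveElevator runs a timeline that lerps the CurrentFloor component from the stored start location to the selected floor marker's height, keeping X and Y.
; When finished, it saves the mesh's new start location and re-enables interaction.
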(event Custom|MoveElevator
  (bind _alpha (Timeline|TL_MoveElevator PlayFromStart)
    (:Update
      (bind _newlocation (CallFunction|SetLocationBasedonSelectedFloor _alpha))
      (Transformation|SetWorldLocation (Variables|Default|GetCurrentFloor) _newlocation false false))
    (:Finished
      (CallFunction|SetNewStartLocation)
      (Variables|Default|SetCanInteract true))))

(event EventInteract
  (bind _returnvalue (Game|GetPlayerController 0))
  (if (Variables|Default|GetCanInteract)
    (Variables|Default|SetCanInteract false)
    (bind _returnvalue_2 (UserInterface|CreateWidget "/Game/ChrisStuff/WBP_FloorSelect.WBP_FloorSelect_C"))
    (bind _output_get (Variables|Default|SetFloorSelectWidget _returnvalue_2))
    (UserInterface|Viewport|AddtoViewport _output_get 0)
    (Input|SetInputModeUIOnly _returnvalue _output_get "DoNotLock" false)
    (Variables|/Script/Engine.PlayerController|SetbShowMouseCursor _returnvalue true)))

(fn ConstructionScript
  (CallFunction|SetNewStartLocation))

(fn SetLocationBasedonSelectedFloor
  (params (Alpha :type Float%20%28single-precision%29))
  (bind _startlocation (Variables|Default|GetStartLocation))
  (bind (_x _y _z) (Math|Vector|BreakVector _startlocation))
  (switch Utilities|FlowControl|Switch|SwitchonE_Floor (Variables|Default|GetFloor)
    (:NewEnumerator0
      (LocalVariables|SetZLocation (.z (Transformation|GetWorldLocation (Variables|Default|GetFloor%201)))))
    (:NewEnumerator1
      (LocalVariables|SetZLocation (.z (Transformation|GetWorldLocation (Variables|Default|GetFloor2)))))
    (:NewEnumerator2
      (LocalVariables|SetZLocation (.z (Transformation|GetWorldLocation (Variables|Default|GetFloor3))))))
  (return (Math|Vector|Lerp(Vector) (Math|Vector|MakeVector _x _y _z) (Math|Vector|MakeVector _x _y (LocalVariables|GetZLocation)) Alpha)))

(fn SetNewStartLocation
  (Variables|Default|SetStartLocation (Transformation|GetWorldLocation (Variables|Default|GetElevatorMesh))))