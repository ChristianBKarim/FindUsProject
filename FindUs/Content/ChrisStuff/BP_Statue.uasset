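; BP_Statue is a green-tinted radiation hazard that rates how close the player is and picks a matching damage value.
; A sphere sized by RadiationRadius enables Tick only while the player overlaps it.
; Each tick maps player distance through fixed thresholds to a Safe, Caution, Danger or Critical state, whose event updates Damage.
; Damage and proximity are only printed on screen, never applied to the player.
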(event OnComponentBeginOverlap(Sphere)
  (params (OverlappedComponent :type Primitive%20Component%20Object%20Reference) (OtherActor :type Actor%20Object%20Reference) (OtherComp :type Primitive%20Component%20Object%20Reference) (OtherBodyIndex :type Integer) (bFromSweep :type Boolean) (SweepResult :type Hit%20Result%20Structure%20%28by%20ref%29))
  (if (CallFunction|IsPlayer OtherActor)
    (Actor|Tick|SetActorTickEnabled true)))

(event OnComponentEndOverlap(Sphere)
  (params (OverlappedComponent :type Primitive%20Component%20Object%20Reference) (OtherActor :type Actor%20Object%20Reference) (OtherComp :type Primitive%20Component%20Object%20Reference) (OtherBodyIndex :type Integer))
  (if (CallFunction|IsPlayer OtherActor)
    (Actor|Tick|SetActorTickEnabled false)))

(event Custom|OnSafe
  (CallFunction|SetDamage)
  (CallFunction|PrintProximity))

(event Custom|OnCritical
  (CallFunction|SetDamage)
  (CallFunction|PrintProximity))

(event Custom|OnCaution
  (CallFunction|SetDamage)
  (CallFunction|PrintProximity))

(event Custom|OnDanger
  (CallFunction|SetDamage)
  (CallFunction|PrintProximity))

(event EventTick
  (params (DeltaSeconds :type Float%20%28single-precision%29))
  (bind _output_get (Variables|Default|SetDistance (Math|Vector|Distance(Vector) (Transformation|GetActorLocation (Game|Player|GetPlayerPawn 0)) (Transformation|GetActorLocation))))
  (Development|PrintString (Utilities|String|ToString(Float) _output_get) true true "(R=0.000000,G=0.660000,B=1.000000,A=1.000000)" 2.0 "fwd")
  (CallFunction|SetDamageAccordingtoProximity))

(event EventBeginPlay
  (Actor|Tick|SetActorTickEnabled false))

(fn ConstructionScript
  (Components|Sphere|SetSphereRadius (Variables|Default|GetSphere) (Variables|Default|GetRadiationRadius) true)
  (Rendering|Material|SetColorParameterValueonMaterials (Variables|Default|GetStaticMesh) "Color" "(R=0.001959,G=0.260417,B=0.035351,A=1.000000)"))

(fn SetDamage
  (Variables|Default|SetDamage (Utilities|Select :Index (Variables|Default|GetProximity) :NewEnumerator0 0.0 :NewEnumerator3 5.0 :NewEnumerator1 2e+01 :NewEnumerator2 35.0))
  (Development|PrintString (Utilities|String|Append "Damage:" (Utilities|String|ToString(Float) (Variables|Default|GetDamage))) true true "(R=0.000000,G=0.660000,B=1.000000,A=1.000000)" 2.0 "dmg"))

(fn PrintProximity
  (switch Utilities|FlowControl|Switch|SwitchonE_DangerRadius (Variables|Default|GetProximity)
    (:NewEnumerator0
      (Development|PrintString "safe" true true "(R=0.000000,G=0.660000,B=1.000000,A=1.000000)" 0.2 "Safe"))
    (:NewEnumerator3
      (Development|PrintString "Caution" true true "(R=0.000000,G=0.660000,B=1.000000,A=1.000000)" 0.2 "Caution"))
    (:NewEnumerator1
      (Development|PrintString "Danger" true true "(R=0.000000,G=0.660000,B=1.000000,A=1.000000)" 0.2 "Danger"))
    (:NewEnumerator2
      (Development|PrintString "Critical!!!" true true "(R=1.000000,G=0.095493,B=0.000000,A=1.000000)" 0.2 "Critical"))))

(fn SetDamageAccordingtoProximity
  (if (> (Variables|Default|GetDistance) 1.15e+03)
    (Variables|Default|SetProximity "NewEnumerator0")
    (CallFunction|OnSafe)
    (elif (and (<= (Variables|Default|GetDistance) 1.15e+03) (> (Variables|Default|GetDistance) 7.5e+02))
      (Variables|Default|SetProximity "NewEnumerator3")
      (CallFunction|OnCaution)
      (elif (and (<= (Variables|Default|GetDistance) 7.5e+02) (> (Variables|Default|GetDistance) 4e+02))
        (Variables|Default|SetProximity "NewEnumerator1")
        (CallFunction|OnDanger)
        (elif (<= (Variables|Default|GetDistance) 4e+02)
          (Variables|Default|SetProximity "NewEnumerator2")
          (CallFunction|OnCritical))))))