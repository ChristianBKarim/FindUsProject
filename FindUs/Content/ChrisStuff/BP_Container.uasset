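; Interactable container that captures an orphan source and closes its lid when the player interacts with it.
; Interacting expands ContainerSphere from zero radius on a timeline while a second timeline moves and rotates the lid shut, then sets IsClosed.
; Any overlap with that growing sphere calls CallSourceCaptured.
; A separate InteractionSphere shows or removes the player character's interaction widget and backs a player-in-range check.
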(event OnComponentBeginOverlap(ContainerSphere)
  (params (OverlappedComponent :type Primitive%20Component%20Object%20Reference) (OtherActor :type Actor%20Object%20Reference) (OtherComp :type Primitive%20Component%20Object%20Reference) (OtherBodyIndex :type Integer) (bFromSweep :type Boolean) (SweepResult :type Hit%20Result%20Structure%20%28by%20ref%29))
  (Default|CallSourceCaptured))

(event OnComponentBeginOverlap(InteractionSphere)
  (params (OverlappedComponent :type Primitive%20Component%20Object%20Reference) (OtherActor :type Actor%20Object%20Reference) (OtherComp :type Primitive%20Component%20Object%20Reference) (OtherBodyIndex :type Integer) (bFromSweep :type Boolean) (SweepResult :type Hit%20Result%20Structure%20%28by%20ref%29))
  (if (CallFunction|IsPlayer OtherActor)
    (UserInterface|Viewport|AddtoViewport (CallFunction|GetInteractionWidget) 0)))

(event OnComponentEndOverlap(InteractionSphere)
  (params (OverlappedComponent :type Primitive%20Component%20Object%20Reference) (OtherActor :type Actor%20Object%20Reference) (OtherComp :type Primitive%20Component%20Object%20Reference) (OtherBodyIndex :type Integer))
  (bind _interactionwidget (CallFunction|GetInteractionWidget))
  (if (CallFunction|IsPlayer OtherActor)
    (Utilities|IsValid _interactionwidget
      (:Is%20Valid
        (Widget|RemovefromParent _interactionwidget)))))

(event EventInteract
  (bind _alpha (Timeline|TL_CaptureOrphanSource PlayFromStart)
    (:Update
      (Components|Sphere|SetSphereRadius (Variables|Default|GetContainerSphere) (Math|Float|Lerp 0.0 3e+02 _alpha) true)
      (if (not (Variables|Default|GetbIsClosed))
        (bind _alpha_2 (Timeline|TL_CloseLid Play)
          (:Update
            (Transformation|SetRelativeLocation (Variables|Default|GetLid) (Math|Vector|Lerp(Vector) "60.000000,0.000000,70.000000" "0.000000,0.000000,85.000000" _alpha_2) false false)
            (Transformation|SetRelativeRotation (Variables|Default|GetLid) (Math|Rotator|Lerp(Rotator) "-30.000000,0.000000,0.000000" "0, 0, 0" _alpha_2) false false))
          (:Finished
            (Variables|Default|SetbIsClosed true)))))))

(fn ConstructionScript)

(fn CheckifPlayerIsinRange
  (return (Collision|IsOverlappingActor (Variables|Default|GetInteractionSphere) (Game|Player|GetPlayerPawn 0) :!class /Script/Engine.PrimitiveComponent)))

(fn GetInteractionWidget
  (return (Variables|/Game/FirstPerson/Blueprints/BP_FirstPersonCharacter.BP_FirstPersonCharacter_C|GetInteractionWidget (.AsBP%20First%20Person%20Character (Utilities|Casting|CastToBP_FirstPersonCharacter (Game|Player|GetPlayerPawn 0))))))