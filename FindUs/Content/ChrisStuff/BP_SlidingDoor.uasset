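; BP_SlidingDoor is a two-panel sliding door that opens while a player is in its sensor area.
; Overlap begin plays the TL_OpenDoor timeline and overlap end reverses it, both only when IsPlayer passes.
; Each timeline update feeds Alpha into OpenDoor, which lerps the left and right panels' relative locations apart along local Y without sweeping.
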(event OnComponentBeginOverlap(SensorArea)
  (params (OverlappedComponent :type Primitive%20Component%20Object%20Reference) (OtherActor :type Actor%20Object%20Reference) (OtherComp :type Primitive%20Component%20Object%20Reference) (OtherBodyIndex :type Integer) (bFromSweep :type Boolean) (SweepResult :type Hit%20Result%20Structure%20%28by%20ref%29))
  (if (CallFunction|IsPlayer OtherActor)
    (bind _alpha (Timeline|TL_OpenDoor Play)
      (:Update
        (CallFunction|OpenDoor _alpha)))))

(event OnComponentEndOverlap(SensorArea)
  (params (OverlappedComponent :type Primitive%20Component%20Object%20Reference) (OtherActor :type Actor%20Object%20Reference) (OtherComp :type Primitive%20Component%20Object%20Reference) (OtherBodyIndex :type Integer))
  (if (CallFunction|IsPlayer OtherActor)
    (bind _alpha (Timeline|TL_OpenDoor Reverse)
      (:Update
        (CallFunction|OpenDoor _alpha)))))

(fn ConstructionScript)

(fn OpenDoor
  (params (Alpha :type Float%20%28double-precision%29))
  (Transformation|SetRelativeLocation (Variables|Default|GetDoorRight) (Math|Vector|Lerp(Vector) "0.000000,-45.000000,0.000000" "0.000000,-90.000000,0.000000" Alpha) false false)
  (Transformation|SetRelativeLocation (Variables|Default|GetDoorLeft) (Math|Vector|Lerp(Vector) "0.000000,45.000000,0.000000" "0.000000,90.000000,0.000000" Alpha) false false))