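; Crowbar pickup actor that gives its item to the player on touch.
; A sphere overlap checks that the other actor is the player, then calls OnPickup.
; OnPickup adds ItemBeingPickedUp to the inventory of player 0's BP_FirstPersonCharacter and destroys the pickup.
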(event OnComponentBeginOverlap(Sphere)
  (params (OverlappedComponent :type Primitive%20Component%20Object%20Reference) (OtherActor :type Actor%20Object%20Reference) (OtherComp :type Primitive%20Component%20Object%20Reference) (OtherBodyIndex :type Integer) (bFromSweep :type Boolean) (SweepResult :type Hit%20Result%20Structure%20%28by%20ref%29))
  (if (CallFunction|IsPlayer OtherActor)
    (CallFunction|OnPickup)))

(fn ConstructionScript
  (|CallParentFunction))

(fn OnPickup
  (Default|AddItem (CallFunction|GetCharacterInventory) (Variables|Default|GetItemBeingPickedUp))
  (Actor|DestroyActor))

(fn GetCharacterInventory
  (return (Variables|/Game/FirstPerson/Blueprints/BP_FirstPersonCharacter.BP_FirstPersonCharacter_C|GetInventory (.AsBP%20First%20Person%20Character (Utilities|Casting|CastToBP_FirstPersonCharacter (Game|GetPlayerCharacter 0))))))