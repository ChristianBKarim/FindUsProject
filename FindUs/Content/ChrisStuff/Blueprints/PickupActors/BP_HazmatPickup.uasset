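; BP_HazmatPickup is a pickup actor that permanently raises the player's maximum radiation value.
; When the player overlaps its Sphere, it adds IncreaseAmount to MaxValue on the first-person character's Radiation, prints the new maximum as debug text, then destroys itself.
; The Radiation reference comes from player pawn 0 cast to BP_FirstPersonCharacter, not from the overlapping actor.
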(event OnComponentBeginOverlap(Sphere)
  (params (OverlappedComponent :type Primitive%20Component%20Object%20Reference) (OtherActor :type Actor%20Object%20Reference) (OtherComp :type Primitive%20Component%20Object%20Reference) (OtherBodyIndex :type Integer) (bFromSweep :type Boolean) (SweepResult :type Hit%20Result%20Structure%20%28by%20ref%29))
  (if (CallFunction|IsPlayer OtherActor)
    (CallFunction|IncreaseMaxValue (Variables|Default|GetIncreaseAmount))
    (CallFunction|DebugMaxRadiation)
    (Actor|DestroyActor)))

(fn ConstructionScript)

(fn IncreaseMaxValue
  (params (Amount :type Float%20%28double-precision%29))
  (bind _radiation (CallFunction|GetPlayerRadiation))
  (Variables|/Game/Components/AC_ValueClamped.AC_ValueClamped_C|SetMaxValue _radiation (+ (Variables|/Game/Components/AC_ValueClamped.AC_ValueClamped_C|GetMaxValue _radiation) Amount)))

(fn GetPlayerRadiation
  (return (Variables|/Game/FirstPerson/Blueprints/BP_FirstPersonCharacter.BP_FirstPersonCharacter_C|GetRadiation (.AsBP%20First%20Person%20Character (Utilities|Casting|CastToBP_FirstPersonCharacter (Game|Player|GetPlayerPawn 0))))))

(fn DebugMaxRadiation
  (Development|PrintString (Utilities|String|Append "Max Radiation:" (Utilities|String|ToString(Float) (Variables|/Game/Components/AC_ValueClamped.AC_ValueClamped_C|GetMaxValue (CallFunction|GetPlayerRadiation))))))