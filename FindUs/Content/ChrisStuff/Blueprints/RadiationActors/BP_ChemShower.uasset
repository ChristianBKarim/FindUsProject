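; BP_ChemShower is a decontamination shower actor that lowers the player's radiation while they stand in its ShowerArea.
; Player overlap starts a looping timer that calls RecoverRad, which decreases the Radiation value on BP_FirstPersonCharacter in fixed steps and prints a debug string.
; The timer is cleared when the player leaves the area or radiation reaches its minimum.
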(event OnComponentBeginOverlap(ShowerArea)
  (params (OverlappedComponent :type Primitive%20Component%20Object%20Reference) (OtherActor :type Actor%20Object%20Reference) (OtherComp :type Primitive%20Component%20Object%20Reference) (OtherBodyIndex :type Integer) (bFromSweep :type Boolean) (SweepResult :type Hit%20Result%20Structure%20%28by%20ref%29))
  (if (CallFunction|IsPlayer OtherActor)
    (bind _returnvalue (Utilities|Time|SetTimerbyFunctionName 0 "RecoverRad" 0.4 true))
    (Variables|Default|SetRecoverRadTimerHandle _returnvalue)))

(event OnComponentEndOverlap(ShowerArea)
  (params (OverlappedComponent :type Primitive%20Component%20Object%20Reference) (OtherActor :type Actor%20Object%20Reference) (OtherComp :type Primitive%20Component%20Object%20Reference) (OtherBodyIndex :type Integer))
  (if (CallFunction|IsPlayer OtherActor)
    (Utilities|Time|ClearandInvalidateTimerbyHandle (Variables|Default|GetRecoverRadTimerHandle))))

(fn ConstructionScript)

(fn RecoverRad
  (bind _returnvalue (Game|Player|GetPlayerPawn 0))
  (bind _asbp_first_person_character (Utilities|Casting|CastToBP_FirstPersonCharacter _returnvalue))
  (bind _radiation (Variables|/Game/FirstPerson/Blueprints/BP_FirstPersonCharacter.BP_FirstPersonCharacter_C|GetRadiation _asbp_first_person_character))
  (Default|ChangeCurrentValue _radiation false 1e+01)
  (Development|PrintString "Hello")
  (if (<= (Default|GetCurrentValue _radiation) (Variables|/Game/Components/AC_ValueClamped.AC_ValueClamped_C|GetMinValue _radiation))
    (Utilities|Time|ClearandInvalidateTimerbyHandle (Variables|Default|GetRecoverRadTimerHandle))))