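; Orphan radiation source that damages the player within its radius until captured through BP_Container, then destroys itself.
; Overlapping the sphere enables Tick, which sorts player distance into proximity tiers derived from CriticalDistance, setting damage and printing debug text.
; Looping timers apply that damage and update the Geiger counter and post-process film grain by tier.
; Leaving or capture stops Tick and timers and resets the feedback.
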(event OnComponentBeginOverlap(RadiationReach)
  (params (OverlappedComponent :type Primitive%20Component%20Object%20Reference) (OtherActor :type Actor%20Object%20Reference) (OtherComp :type Primitive%20Component%20Object%20Reference) (OtherBodyIndex :type Integer) (bFromSweep :type Boolean) (SweepResult :type Hit%20Result%20Structure%20%28by%20ref%29))
  (if (CallFunction|IsPlayer OtherActor)
    (Actor|Tick|SetActorTickEnabled true)
    (bind _returnvalue (Utilities|Time|SetTimerbyFunctionName 0 "DamagePlayer" 1.2 true))
    (Variables|Default|SetDamageHandle _returnvalue)
    (bind _returnvalue_2 (Actor|GetActorOfClass "/Game/FirstPerson/Blueprints/BP_GeigerCounter.BP_GeigerCounter_C"))
    (Variables|Default|SetGeigerCounterRef _returnvalue_2)
    (bind _returnvalue_3 (Utilities|Time|SetTimerbyEvent (EventDispatchers|CreateEvent :!event Custom|InRadiationRadiusEvent) 1.0 true))
    (Variables|Default|SetGeigerCounterHandle _returnvalue_3)))

(event OnComponentEndOverlap(RadiationReach)
  (params (OverlappedComponent :type Primitive%20Component%20Object%20Reference) (OtherActor :type Actor%20Object%20Reference) (OtherComp :type Primitive%20Component%20Object%20Reference) (OtherBodyIndex :type Integer))
  (if (CallFunction|IsPlayer OtherActor)
    (CallFunction|PlayerAwayfromDanger)))

(event Custom|OnSafe
  (CallFunction|SetDamage)
  (CallFunction|DebugProximity))

(event Custom|OnCritical
  (CallFunction|SetDamage)
  (CallFunction|DebugProximity))

(event Custom|OnCaution
  (CallFunction|SetDamage)
  (CallFunction|DebugProximity))

(event Custom|InRadiationRadiusEvent
  (CallFunction|CallDeviceinRadiusDispatch)
  (Utilities|IsValid (Variables|Default|GetPostProcessRef)
    (:Is%20Valid
      (CallFunction|UpdatePostProcessVolume (Variables|Default|GetProximity)))))

(event Custom|OnDanger
  (CallFunction|SetDamage)
  (CallFunction|DebugProximity))

(event Custom|OnCaptured
  (if (not (Variables|Default|GetbIsCaptured))
    (Variables|Default|SetbIsCaptured true)
    (CallFunction|PlayerAwayfromDanger)
    (Actor|DestroyActor)))

(event EventTick
  (params (DeltaSeconds :type Float%20%28single-precision%29))
  (bind _output_get (Variables|Default|SetDistance (Math|Vector|Distance(Vector) (Transformation|GetActorLocation (Game|Player|GetPlayerPawn 0)) (Transformation|GetActorLocation))))
  (Development|PrintString (Utilities|String|ToString(Float) _output_get) true true "(R=0.000000,G=0.660000,B=1.000000,A=1.000000)" 2.0 "fwd")
  (CallFunction|SetDamageAccordingtoProximity))

(event EventBeginPlay
  (Actor|Tick|SetActorTickEnabled false)
  (bind _returnvalue (Actor|GetActorOfClass "/Game/ChrisStuff/Blueprints/RadiationActors/BP_Container.BP_Container_C"))
  (bind _output_get (Variables|Default|SetContainerRef _returnvalue))
  (EventDispatchers|BindEventtoSourceCaptured _output_get (EventDispatchers|CreateEvent :!event Custom|OnCaptured)))

(fn ConstructionScript
  (Components|Sphere|SetSphereRadius (Variables|Default|GetRadiationReach) (Variables|Default|GetRadiationRadius) true)
  (Rendering|Material|SetColorParameterValueonMaterials (Variables|Default|GetStaticMesh) "Color" "(R=0.001959,G=0.260417,B=0.035351,A=1.000000)")
  (Variables|Default|SetDangerDistance (* (Variables|Default|GetCriticalDistance) 1.8))
  (Variables|Default|SetSafeDistance (* (Variables|Default|GetCriticalDistance) 2.8)))

(fn SetDamage
  (Variables|Default|SetDamage (Utilities|Select :Index (Variables|Default|GetProximity) :NewEnumerator4 0.0 :NewEnumerator0 3.0 :NewEnumerator3 1e+01 :NewEnumerator1 2e+01 :NewEnumerator2 35.0))
  (Development|PrintString (Utilities|String|Append "Damage:" (Utilities|String|ToString(Float) (Variables|Default|GetDamage))) true true "(R=0.000000,G=0.660000,B=1.000000,A=1.000000)" 2.0 "dmg"))

(fn DebugProximity
  (switch Utilities|FlowControl|Switch|SwitchonE_DangerRadius (Variables|Default|GetProximity)
    (:NewEnumerator0
      (Development|PrintString "safe" true true "(R=0.000000,G=0.660000,B=1.000000,A=1.000000)" 0.2 "Safe"))
    (:NewEnumerator3
      (Development|PrintString "Caution" true true "(R=0.000000,G=0.660000,B=1.000000,A=1.000000)" 0.2 "Caution"))
    (:NewEnumerator1
      (Development|PrintString "Danger" true true "(R=0.000000,G=0.660000,B=1.000000,A=1.000000)" 0.2 "Danger"))
    (:NewEnumerator2
      (Development|PrintString "Critical!!!" true true "(R=1.000000,G=0.095493,B=0.000000,A=1.000000)" 0.2 "Critical"))))

(fn SetDamageAccordingtoProximity
  (if (> (Variables|Default|GetDistance) (Variables|Default|GetSafeDistance))
    (Variables|Default|SetProximity "NewEnumerator0")
    (CallFunction|OnSafe)
    (elif (and (<= (Variables|Default|GetDistance) (Variables|Default|GetSafeDistance)) (> (Variables|Default|GetDistance) (Variables|Default|GetDangerDistance)))
      (Variables|Default|SetProximity "NewEnumerator3")
      (CallFunction|OnCaution)
      (elif (and (<= (Variables|Default|GetDistance) (Variables|Default|GetDangerDistance)) (> (Variables|Default|GetDistance) (Variables|Default|GetCriticalDistance)))
        (Variables|Default|SetProximity "NewEnumerator1")
        (CallFunction|OnDanger)
        (elif (<= (Variables|Default|GetDistance) (Variables|Default|GetCriticalDistance))
          (Variables|Default|SetProximity "NewEnumerator2")
          (CallFunction|OnCritical))))))

(fn DamagePlayer
  (Game|Damage|ApplyDamage (Game|Player|GetPlayerPawn 0) (Variables|Default|GetDamage) 0 0))

(fn RecoverRad
  (bind _returnvalue (Game|Player|GetPlayerPawn 0))
  (bind _asbp_first_person_character (Utilities|Casting|CastToBP_FirstPersonCharacter _returnvalue))
  (bind _radiation (Variables|/Game/FirstPerson/Blueprints/BP_FirstPersonCharacter.BP_FirstPersonCharacter_C|GetRadiation _asbp_first_person_character))
  (Default|ChangeCurrentValue _radiation false 1e+01)
  (if (<= (Default|GetCurrentValue _radiation) (Variables|/Game/Components/AC_ValueClamped.AC_ValueClamped_C|GetMinValue _radiation))
    _))

(fn CallDeviceinRadiusDispatch
  (if (or (Utilities|Enum|Equal(Enum) (Variables|Default|GetProximity) "NewEnumerator0") (Utilities|Enum|Equal(Enum) (Variables|Default|GetProximity) "NewEnumerator3"))
    (Default|CallDeviceinRadius (Variables|Default|GetGeigerCounterRef) true false)
    (elif (or (Utilities|Enum|Equal(Enum) (Variables|Default|GetProximity) "NewEnumerator1") (Utilities|Enum|Equal(Enum) (Variables|Default|GetProximity) "NewEnumerator2"))
      (Default|CallDeviceinRadius (Variables|Default|GetGeigerCounterRef) true true))))

(fn UpdatePostProcessVolume
  (params (Proximity :type E_DangerRadius%20Enum :default "NewEnumerator0"))
  (switch Utilities|FlowControl|Switch|SwitchonE_DangerRadius Proximity
    (:NewEnumerator4
      (Utilities|Struct|SetmembersinPostProcessSettings (Variables|/Script/Engine.PostProcessVolume|GetSettings (Variables|Default|GetPostProcessRef)) 0.0 0.0))
    (:NewEnumerator0
      (Utilities|Struct|SetmembersinPostProcessSettings (Variables|/Script/Engine.PostProcessVolume|GetSettings (Variables|Default|GetPostProcessRef)) 0.5 1.5))
    (:NewEnumerator3
      (Utilities|Struct|SetmembersinPostProcessSettings (Variables|/Script/Engine.PostProcessVolume|GetSettings (Variables|Default|GetPostProcessRef)) 1.0 1.5))
    (:NewEnumerator1
      (Utilities|Struct|SetmembersinPostProcessSettings (Variables|/Script/Engine.PostProcessVolume|GetSettings (Variables|Default|GetPostProcessRef)) 1.0 2.5))
    (:NewEnumerator2
      (Utilities|Struct|SetmembersinPostProcessSettings (Variables|/Script/Engine.PostProcessVolume|GetSettings (Variables|Default|GetPostProcessRef)) 1.0 4.0))))

(fn PlayerAwayfromDanger
  (Actor|Tick|SetActorTickEnabled false)
  (Utilities|Time|ClearandInvalidateTimerbyHandle (Variables|Default|GetDamageHandle))
  (Utilities|Time|ClearandInvalidateTimerbyHandle (Variables|Default|GetGeigerCounterHandle))
  (Default|DeviceinRadiusEvent (Variables|Default|GetGeigerCounterRef) false false)
  (CallFunction|UpdatePostProcessVolume "NewEnumerator4"))