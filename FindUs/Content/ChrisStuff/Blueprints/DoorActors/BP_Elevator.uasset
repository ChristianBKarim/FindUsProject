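; Elevator actor with a sliding door that travels between three floors.
; Interact disables player input and opens the WBP_FloorSelect widget in UI-only mode with the mouse cursor.
; A door timeline slides the door and triggers the move timeline on each update, lerping height toward the selected floor marker's Z.
; On arrival it stores the new start location and floor number, re-enables interaction, and reverses the door timeline if DoorIsClosed is set.
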(event Custom|MoveElevator
  (bind _alpha (Timeline|TL_MoveElevator PlayFromStart)
    (:Update
      (bind _newlocation (CallFunction|SetLocationBasedonSelectedFloor _alpha))
      (Transformation|SetWorldLocation (Variables|Default|GetCurrentFloor) _newlocation false false))
    (:Finished
      (CallFunction|SetNewStartLocation)
      (Variables|Default|SetCanInteract true)
      (CallFunction|SetCurrrentFloor)
      (if (Variables|Default|GetDoorIsClosed)
        (CallFunction|CloseDoor)
        (Development|PrintString (Utilities|String|Append "Current Floor: " (Utilities|String|ToString(Integer) (Variables|Default|GetFloorCurrentlyOn))))))))

(event Custom|MoveDoor
  (if (Variables|Default|GetDoorIsClosed)
    (bind _alpha (Timeline|TL_MoveDoor Reverse)
      (:Update
        (Transformation|SetRelativeLocation (Variables|Default|GetDoor) (Math|Vector|Lerp(Vector) "77.777777,209.000000,0.000000" "77.777777,0.000000,0.000000" _alpha) false false)
        (CallFunction|MoveElevator))
      (:Finished
        (Variables|Default|SetDoorIsClosed (not (Variables|Default|GetDoorIsClosed)))))
    (else
      (Timeline|TL_MoveDoor Play))))

(event Custom|CloseDoor
  (bind _alpha (Timeline|TL_MoveDoor Reverse)
    (:Update
      (Transformation|SetRelativeLocation (Variables|Default|GetDoor) (Math|Vector|Lerp(Vector) "77.777777,209.000000,0.000000" "77.777777,0.000000,0.000000" _alpha) false false)
      (CallFunction|MoveElevator))
    (:Finished
      (Variables|Default|SetDoorIsClosed (not (Variables|Default|GetDoorIsClosed))))))

(event EventBeginPlay
  (CallFunction|SetCurrrentFloor))

(event EventInteract
  (bind _returnvalue (Game|GetPlayerController 0))
  (if (Variables|Default|GetCanInteract)
    (Variables|Default|SetCanInteract false)
    (Input|DisableInput (Game|Player|GetPlayerPawn 0) 0)
    (bind _returnvalue_2 (UserInterface|CreateWidget "/Game/ChrisStuff/Blueprints/WidgetBlueprints/WBP_FloorSelect.WBP_FloorSelect_C"))
    (bind _output_get (Variables|Default|SetFloorSelectWidget _returnvalue_2))
    (UserInterface|Viewport|AddtoViewport _output_get 0)
    (Input|SetInputModeUIOnly _returnvalue _output_get "DoNotLock" false)
    (Variables|/Script/Engine.PlayerController|SetbShowMouseCursor _returnvalue true)))

(fn ConstructionScript
  (CallFunction|SetNewStartLocation))

(fn SetLocationBasedonSelectedFloor
  (params (Alpha :type Float%20%28single-precision%29))
  (bind _startlocation (Variables|Default|GetStartLocation))
  (bind (_x _y _z) (Math|Vector|BreakVector _startlocation))
  (switch Utilities|FlowControl|Switch|SwitchonE_Floor (Variables|Default|GetFloor)
    (:NewEnumerator0
      (LocalVariables|SetZLocation (.z (Transformation|GetWorldLocation (Variables|Default|GetFloor1)))))
    (:NewEnumerator1
      (LocalVariables|SetZLocation (.z (Transformation|GetWorldLocation (Variables|Default|GetFloor2)))))
    (:NewEnumerator2
      (LocalVariables|SetZLocation (.z (Transformation|GetWorldLocation (Variables|Default|GetFloor3))))))
  (return (Math|Vector|Lerp(Vector) (Math|Vector|MakeVector _x _y _z) (Math|Vector|MakeVector _x _y (LocalVariables|GetZLocation)) Alpha)))

(fn SetNewStartLocation
  (Variables|Default|SetStartLocation (Transformation|GetWorldLocation (Variables|Default|GetElevatorMesh))))

(fn SetCurrrentFloor
  (switch Utilities|FlowControl|Switch|SwitchonE_Floor (Variables|Default|GetFloor)
    (:NewEnumerator0
      (Variables|Default|SetFloorCurrentlyOn 1))
    (:NewEnumerator1
      (Variables|Default|SetFloorCurrentlyOn 2))
    (:NewEnumerator2
      (Variables|Default|SetFloorCurrentlyOn 3))))