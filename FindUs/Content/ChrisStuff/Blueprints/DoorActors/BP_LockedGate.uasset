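; BP_LockedGate is a double gate that stays locked until the player has a required inventory item.
; A trigger box toggles interaction and an "Open Gate" prompt widget.
; Interacting with the item plays shotgun sounds, then knocks the lock off with a physics impulse, unlocks the gate and destroys the lock.
; A later interaction plays a timeline that swings both halves open through rotation lerps.
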(event OnComponentBeginOverlap(Box)
  (params (OverlappedComponent :type Primitive%20Component%20Object%20Reference) (OtherActor :type Actor%20Object%20Reference) (OtherComp :type Primitive%20Component%20Object%20Reference) (OtherBodyIndex :type Integer) (bFromSweep :type Boolean) (SweepResult :type Hit%20Result%20Structure%20%28by%20ref%29))
  (if (CallFunction|IsPlayer OtherActor)
    (CallFunction|EnableInteraction)))

(event OnComponentEndOverlap(Box)
  (params (OverlappedComponent :type Primitive%20Component%20Object%20Reference) (OtherActor :type Actor%20Object%20Reference) (OtherComp :type Primitive%20Component%20Object%20Reference) (OtherBodyIndex :type Integer))
  (if (CallFunction|IsPlayer OtherActor)
    (CallFunction|DisableInteraction)))

(event Custom|ShootLock
  (bind _lock (Variables|Default|GetLock))
  (Audio|PlaySound2D "/Game/ChrisStuff/SFX/SW_ShotgunCocking.SW_ShotgunCocking" 1.0 1.0 0.0 0 0)
  (Utilities|FlowControl|Delay 1.2)
  (Audio|PlaySound2D "/Game/ChrisStuff/SFX/SW_ShotgunFired.SW_ShotgunFired" 1.0 1.0 0.0 0 0)
  (Utilities|FlowControl|Delay 0.2)
  (Physics|SetSimulatePhysics _lock true)
  (Physics|AddImpulse _lock "0.000000,-300.000000,500.000000" "None" false)
  (Variables|Default|SetDoorIsLocked false)
  (Utilities|FlowControl|Delay 1.0)
  (Components|DestroyComponent (Variables|Default|GetLock)))

(event Custom|OpenGate
  (bind _alpha (Timeline|TL_OpenGate Play)
    (:Update
      (CallFunction|OpentheGate _alpha))))

(event EventInteract
  (bind _inventory (CallFunction|GetPlayerInventory))
  (if (and (Variables|Default|GetbCanInteract) (Variables|Default|GetDoorIsLocked))
    (Utilities|IsValid _inventory
      (:Is%20Valid
        (bind _returnvalue (Default|HasItem _inventory (Variables|Default|GetItemNeeded)))
        (if _returnvalue
          (CallFunction|ShootLock))))
    (elif (not (Variables|Default|GetDoorIsLocked))
      (CallFunction|OpenGate))))

(fn ConstructionScript)

(fn EnableInteraction
  (Variables|Default|SetbCanInteract true)
  (bind _returnvalue (UserInterface|CreateWidget "/Game/ChrisStuff/Blueprints/WidgetBlueprints/WBP_CanInteract.WBP_CanInteract_C"))
  (bind _output_get (Variables|Default|SetInteractWidget _returnvalue))
  (Variables|/Game/ChrisStuff/Blueprints/WidgetBlueprints/WBP_CanInteract.WBP_CanInteract_C|SetText _output_get "Open Gate")
  (UserInterface|Viewport|AddtoViewport (Variables|Default|GetInteractWidget) 0))

(fn DisableInteraction
  (Variables|Default|SetbCanInteract false)
  (Widget|RemovefromParent (Variables|Default|GetInteractWidget)))

(fn GetPlayerInventory
  (return (Variables|/Game/FirstPerson/Blueprints/BP_FirstPersonCharacter.BP_FirstPersonCharacter_C|GetInventory (.AsBP%20First%20Person%20Character (Utilities|Casting|CastToBP_FirstPersonCharacter (Game|Player|GetPlayerPawn 0))))))

(fn OpentheGate
  (params (Alpha :type Float%20%28double-precision%29))
  (Transformation|SetRelativeRotation (Variables|Default|GetGateLeft) (Math|Rotator|Lerp(Rotator) "0.000000,180.000000,0.000000" "0.000000,90.000000,0.000000" Alpha) false false)
  (Transformation|SetRelativeRotation (Variables|Default|GetGateRight) (Math|Rotator|Lerp(Rotator) "0, 0, 0" "0.000000,90.000000,0.000000" Alpha) false false))