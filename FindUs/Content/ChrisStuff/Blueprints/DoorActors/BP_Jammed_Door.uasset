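; BP_Jammed_Door is a jammed door that the player pries open when their inventory holds the required ItemNeeded.
; Its Box overlap shows a "Pry open" widget and enables interaction until the player leaves, skipping the prompt once the door is open.
; A successful Interact runs a timeline that swings the door open and disables the DoorFrame collision.
; A PlaySound2D node exists but is unconnected.
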(event OnComponentBeginOverlap(Box)
  (params (OverlappedComponent :type Primitive%20Component%20Object%20Reference) (OtherActor :type Actor%20Object%20Reference) (OtherComp :type Primitive%20Component%20Object%20Reference) (OtherBodyIndex :type Integer) (bFromSweep :type Boolean) (SweepResult :type Hit%20Result%20Structure%20%28by%20ref%29))
  (if (CallFunction|IsPlayer OtherActor)
    (if (not (Variables|Default|GetbDoorAlreadyOpen))
      (bind _returnvalue (UserInterface|CreateWidget "/Game/ChrisStuff/Blueprints/WidgetBlueprints/WBP_CanInteract.WBP_CanInteract_C"))
      (bind _output_get (Variables|Default|SetInteractWidget _returnvalue))
      (Variables|/Game/ChrisStuff/Blueprints/WidgetBlueprints/WBP_CanInteract.WBP_CanInteract_C|SetText _output_get "Pry open")
      (UserInterface|Viewport|AddtoViewport _output_get 0)
      (Variables|Default|SetbCanInteract true))))

(event OnComponentEndOverlap(Box)
  (params (OverlappedComponent :type Primitive%20Component%20Object%20Reference) (OtherActor :type Actor%20Object%20Reference) (OtherComp :type Primitive%20Component%20Object%20Reference) (OtherBodyIndex :type Integer))
  (if (CallFunction|IsPlayer OtherActor)
    (Widget|RemovefromParent (Variables|Default|GetInteractWidget))
    (Variables|Default|SetbCanInteract false)))

(event Custom|DoorBreaksOpen
  (Variables|Default|SetbDoorAlreadyOpen true)
  (bind _alpha (Timeline|TL_MoveDoor Play)
    (:Update
      (Transformation|SetRelativeRotation (Variables|Default|GetDoor) (Math|Rotator|Lerp(Rotator) "0, 0, 0" "0.000000,-80.000000,0.000000" _alpha) false false)
      (Collision|SetCollisionEnabled (Variables|Default|GetDoorFrame) "NoCollision"))))

(event EventInteract
  (if (Variables|Default|GetbCanInteract)
    (bind _returnvalue (Default|HasItem (CallFunction|GetPlayerInventory) (Variables|Default|GetItemNeeded)))
    (if _returnvalue
      (CallFunction|DoorBreaksOpen))))

(fn ConstructionScript)

(fn GetPlayerInventory
  (return (Variables|/Game/FirstPerson/Blueprints/BP_FirstPersonCharacter.BP_FirstPersonCharacter_C|GetInventory (.AsBP%20First%20Person%20Character (Utilities|Casting|CastToBP_FirstPersonCharacter (Game|GetPlayerCharacter 0))))))