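; Elevator call button that, on Interact, summons its linked elevator to the button's floor.
; If the elevator allows interaction, it locks it, tints the button green and sets the elevator's target floor to CurrentFloor.
; After a short delay it starts MoveElevator and resets the button color to white.
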(event EventInteract
  (bind _elevator (Variables|Default|GetElevator))
  (if (Variables|/Game/ChrisStuff/BP_Elevator.BP_Elevator_C|GetCanInteract _elevator)
    (Variables|/Game/ChrisStuff/BP_Elevator.BP_Elevator_C|SetCanInteract _elevator false)
    (Rendering|Material|SetColorParameterValueonMaterials (Variables|Default|GetButton) "Color" "(R=0.000000,G=1.000000,B=0.127104,A=1.000000)")
    (Variables|/Game/ChrisStuff/BP_Elevator.BP_Elevator_C|SetFloor (Variables|Default|GetElevator) (Variables|Default|GetCurrentFloor))
    (Utilities|FlowControl|Delay 0.3)
    (Default|MoveElevator (Variables|Default|GetElevator))
    (Rendering|Material|SetColorParameterValueonMaterials (Variables|Default|GetButton) "Color" "(R=1.000000,G=1.000000,B=1.000000,A=1.000000)")))

(fn ConstructionScript)