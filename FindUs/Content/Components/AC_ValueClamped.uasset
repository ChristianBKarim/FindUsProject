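; Reusable clamped-float component for stats shown in the UI, such as health or radiation.
; BeginPlay initializes the value to current, min or max based on DefaultInitialValue.
; ChangeCurrentValue adds or subtracts an amount, clamps it to range, then refreshes the UI.
; UpdateUI sends value divided by max through an interface reference, with an enum choosing the health or rad update.
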(event Custom|ChangeCurrentValue
  (params (ShouldIncrease? :type Boolean) (Amount :type Float%20%28double-precision%29))
  (if ShouldIncrease?
    (Variables|Default|SetCurrentValue (+ (Variables|Default|GetCurrentValue) Amount))
    (else
      (Variables|Default|SetCurrentValue (- (Variables|Default|GetCurrentValue) Amount))))
  (CallFunction|ValidateCurrentValue)
  (CallFunction|UpdateUI))

(event EventBeginPlay
  (Variables|Default|SetCurrentValue (Utilities|Select :Index (Variables|Default|GetDefaultInitialValue) :NewEnumerator0 (Variables|Default|GetCurrentValue) :NewEnumerator1 (Variables|Default|GetMinValue) :NewEnumerator2 (Variables|Default|GetMaxValue))))

(fn ValidateCurrentValue
  (Variables|Default|SetCurrentValue (Math|Float|Clamp(Float) (Variables|Default|GetCurrentValue) (Variables|Default|GetMinValue) (Variables|Default|GetMaxValue))))

(fn GetCurrentValueasPercent
  (return (/ (Variables|Default|GetCurrentValue) (Variables|Default|GetMaxValue))))

(fn UpdateUI
  (if (Utilities|IsValidInterface (Variables|Default|GetUIRef))
    (if (Utilities|Enum|Equal(Enum) (Variables|Default|GetUIElementToUpdate) "NewEnumerator0")
      (Default|UpdateFloatValueHealth (Variables|Default|GetUIRef) "NewEnumerator0" (CallFunction|GetCurrentValueasPercent))
      (elif (Utilities|Enum|Equal(Enum) (Variables|Default|GetUIElementToUpdate) "NewEnumerator1")
        (Default|UpdateFloatValueRad (Variables|Default|GetUIRef) "NewEnumerator1" (CallFunction|GetCurrentValueasPercent))))))

(fn GetCurrentValue
  (return (Variables|Default|GetCurrentValue)))