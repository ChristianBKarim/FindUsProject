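; Inventory actor component that stores items in an Items array.
; AddItem appends the given item without any checks and always returns true.
; HasItem compares items by ItemName, but returns inside the loop, so only the first element is ever checked.
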(fn AddItem
  (params (ItemToAdd :type DS%20Inventory%20Item%20Structure))
  (Utilities|Array|Add (Variables|Default|GetItems) ItemToAdd)
  (return true))

(fn HasItem
  (params (ItemToCheck :type DS%20Inventory%20Item%20Structure))
  (for _array_element (Variables|Default|GetItems)
    (return (Utilities|Enum|Equal(Enum) (Utilities|Struct|BreakDS_InventoryItem _array_element) (Utilities|Struct|BreakDS_InventoryItem ItemToCheck)))))