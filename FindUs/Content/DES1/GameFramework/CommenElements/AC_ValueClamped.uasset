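; AC_ValueClamped is a component that holds a numeric value kept between a minimum and maximum.
; BeginPlay picks the starting value from a default, minimum or maximum option, and ChangeCurrentValue adds or subtracts an amount.
; Both then call ValidateCurrentValue, which clamps and prints the result.
; Getters return the raw value or its ratio to the maximum, while UpdateUI is an unfinished interface-check stub.
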(event Custom|ChangeCurrentValue
  (params (ShouldIncrease :type Boolean) (Amount :type Float%20%28double-precision%29))
  (if ShouldIncrease
    (Variables|Default|SetCurrentValue (+ (Variables|Default|GetCurrentValue) Amount))
    (else
      (Variables|Default|SetCurrentValue (- (Variables|Default|GetCurrentValue) Amount))))
  (CallFunction|ValidateCurrentValue))

(event EventBeginPlay
  (Variables|Default|SetCurrentValue (Utilities|Select :Index (Variables|Default|GetDefaultInitialValue) :NewEnumerator0 (Variables|Default|GetCurrentValue) :NewEnumerator1 (Variables|Default|GetMinValue) :NewEnumerator2 (Variables|Default|GetMaxValue)))
  (CallFunction|ValidateCurrentValue))

(fn ValidateCurrentValue
  (bind _output_get (Variables|Default|SetCurrentValue (Math|Float|Clamp(Float) (Variables|Default|GetCurrentValue) (Variables|Default|GetMinValue) (Variables|Default|GetMaxValue))))
  (Development|PrintString (Utilities|String|ToString(Float) _output_get)))

(fn GetCurrentValue
  (return (Variables|Default|GetCurrentValue)))

(fn UpdateUI
  (if (Utilities|IsValidInterface (Variables|Default|GetUIRefference))
    _))

(fn GetCurrentasPercent
  (return (/ (Variables|Default|GetCurrentValue) (Variables|Default|GetMaxValue))))