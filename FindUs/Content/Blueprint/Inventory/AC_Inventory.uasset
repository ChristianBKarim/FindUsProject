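; AC_Inventory is an inventory component that keeps items and consumables in two separate arrays.
; Add functions look up an entry by Name, then either increment its Amount or append a new entry and return true.
; Has functions wrap the Find lookups, which use -1 as not found.
; RemoveItem is an empty stub, and FindItem's loop has no array connected, unlike FindConsumable, so it never searches Items.
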(event EventBeginPlay)

(event EventTick
  (params (DeltaSeconds :type Float%20%28single-precision%29)))

(fn AddItem
  (params (ItemToAdd :type DS%20Inventory%20Structure))
  (bind _output_get (LocalVariables|SetFoundIndex (CallFunction|FindItem ItemToAdd)))
  (if (== _output_get -1)
    (Math|Integer|IncrementInt (.Amount (Utilities|Struct|BreakDS_Inventory ItemToAdd))
      (:%20%20
        (Utilities|Array|Add (Variables|Default|GetItems) ItemToAdd)
        (return true)))
    (else
      (Math|Integer|IncrementInt (.Amount (Utilities|Struct|BreakDS_Inventory (Utilities|Array|Get(acopy) (Variables|Default|GetItems) (LocalVariables|GetFoundIndex))))))))

(fn RemoveItem
  (params (ItemToRemove :type DS%20Inventory%20Structure)))

(fn FindItem
  (params (ItemToFind :type DS%20Inventory%20Structure))
  (bind (_array_element _array_index) (Utilities|Array|ForEachLoopwithBreak 0 :!label _label)
    (:LoopBody
      (if (Utilities|Enum|Equal(Enum) (Utilities|Struct|BreakDS_Inventory _array_element) (Utilities|Struct|BreakDS_Inventory ItemToFind))
        (LocalVariables|SetFoundIndex _array_index)
        (goto _label Break)))
    (:Completed
      (return (LocalVariables|GetFoundIndex)))))

(fn HasItem
  (params (ItemToCheck :type DS%20Inventory%20Structure) (ConsumablesToCheck :type DS%20Consumable%20Structure))
  (return (!= (CallFunction|FindItem ItemToCheck) -1)))

(fn FindConsumable
  (params (ConsumableToFind :type DS%20Consumable%20Structure))
  (bind (_array_element _array_index) (Utilities|Array|ForEachLoopwithBreak (Variables|Default|GetConsumable) :!label _label)
    (:LoopBody
      (if (Utilities|Enum|Equal(Enum) (Utilities|Struct|BreakDS_Consumable _array_element) (Utilities|Struct|BreakDS_Consumable ConsumableToFind))
        (LocalVariables|SetFoundIndex _array_index)
        (goto _label Break)))
    (:Completed
      (return (LocalVariables|GetFoundIndex)))))

(fn AddConsumable
  (params (ConsumableToAdd :type DS%20Consumable%20Structure))
  (bind _output_get (LocalVariables|SetFoundIndex (CallFunction|FindConsumable ConsumableToAdd)))
  (if (== _output_get -1)
    (Math|Integer|IncrementInt (.Amount (Utilities|Struct|BreakDS_Consumable ConsumableToAdd))
      (:%20%20
        (Utilities|Array|Add (Variables|Default|GetConsumable) ConsumableToAdd)
        (return true)))
    (else
      (Math|Integer|IncrementInt (.Amount (Utilities|Struct|BreakDS_Consumable (Utilities|Array|Get(acopy) (Variables|Default|GetConsumable) (LocalVariables|GetFoundIndex))))))))

(fn HasConsumable
  (params (ConsumablesToCheck :type DS%20Consumable%20Structure))
  (return (!= (CallFunction|FindConsumable ConsumablesToCheck) -1)))