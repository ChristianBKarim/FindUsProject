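; BP_HealthPickup is a health pickup that gives the player a consumable on contact.
; When a player overlaps PickupArea, OnPickup casts the local player pawn to BP_FirstPersonCharacter, adds its Consumable to that character's Inventory, and destroys the pickup.
; The construction script runs the parent's setup, then tints the mesh dark red through the Color material parameter.
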(event OnComponentBeginOverlap(PickupArea)
  (params (OverlappedComponent :type Primitive%20Component%20Object%20Reference) (OtherActor :type Actor%20Object%20Reference) (OtherComp :type Primitive%20Component%20Object%20Reference) (OtherBodyIndex :type Integer) (bFromSweep :type Boolean) (SweepResult :type Hit%20Result%20Structure%20%28by%20ref%29))
  (if (CallFunction|IsPlayer OtherActor)
    (CallFunction|OnPickup (Game|Player|GetPlayerPawn 0))))

(fn ConstructionScript
  (|CallParentFunction)
  (Rendering|Material|SetColorParameterValueonMaterials (Variables|Character|GetMesh) "Color" "(R=0.116319,G=0.000000,B=0.000000,A=0.000000)"))

(fn OnPickup
  (params (ActorRef :type Actor%20Object%20Reference))
  (bind _asbp_first_person_character (Utilities|Casting|CastToBP_FirstPersonCharacter ActorRef))
  (Default|AddConsumable (Variables|/Game/FirstPerson/Blueprints/BP_FirstPersonCharacter.BP_FirstPersonCharacter_C|GetInventory _asbp_first_person_character) (Variables|Default|GetConsumable))
  (Actor|DestroyActor))